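; Anim notify state that lets the player steer Free Flow movement with the left stick during an animation.
; Each tick with the stick held, it rotates the input by camera rotation and line-traces a short distance ahead at raised height.
; If unobstructed, it moves the player pawn along that scaled offset over a set time, optionally snapping to floor.
; Weapon-specific tuning, rotation lerp and lock-on range logic are present but disconnected.
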(fn ReceivedNotifyTick
  (params (MeshComp :type Skeletal%20Mesh%20Component%20Object%20Reference) (Animation :type Anim%20Sequence%20Base%20Object%20Reference) (FrameDeltaTime :type Float%20%28single-precision%29))
  (LocalVariables|SetPlayerController (Game|GetPlayerController MeshComp))
  (if (Math|Boolean|ORBoolean (Game|Player|IsInputKeyDown (LocalVariables|GetPlayerController) "Gamepad_LeftStick_Up") (Game|Player|IsInputKeyDown (LocalVariables|GetPlayerController) "Gamepad_LeftStick_Down") (Game|Player|IsInputKeyDown (LocalVariables|GetPlayerController) "Gamepad_LeftStick_Left") (Game|Player|IsInputKeyDown (LocalVariables|GetPlayerController) "Gamepad_LeftStick_Right"))
    (bind _output_get (LocalVariables|SetPlayerPawn (Class|TresGameBlueprintLibrary|GetTresPlayerPawnBase (LocalVariables|GetPlayerController))))
    (LocalVariables|SetCameraManager (Class|TresGameBlueprintLibrary|GetLocalTresCameraManager _output_get))
    (Class|TresGameBlueprintLibrary|TresDelay (LocalVariables|GetPlayerPawn) (+ (Variables|Default|GetTime) 0.001))
    (bind _returnvalue (Collision|LineTraceForObjects (LocalVariables|GetPlayerController) (Math|Vector|MakeVector (.x (Transformation|GetActorLocation (LocalVariables|GetPlayerPawn))) (.y (Transformation|GetActorLocation (LocalVariables|GetPlayerPawn))) (+ (.z (Transformation|GetActorLocation (LocalVariables|GetPlayerPawn))) 75.0)) (Math|Vector|MakeVector (+ (* (.x (Math|Vector|GetForwardVector (Math|Conversions|RotationFromXVector (* (Math|Vector|RotateVector (Math|Vector|MakeVector (.StickY (Class|PlayerController|GetInputAnalogStickState (LocalVariables|GetPlayerController) "CAS_LeftStick")) (.StickX (Class|PlayerController|GetInputAnalogStickState (LocalVariables|GetPlayerController) "CAS_LeftStick")) 0.0) (Transformation|GetActorRotation (LocalVariables|GetCameraManager))) (Math|Vector|MakeVector (Variables|Default|GetLeftRightScale) (Variables|Default|GetForwardBackwardScale) 0.0))))) 75.0) (.x (Transformation|GetActorLocation (LocalVariables|GetPlayerPawn)))) (+ (* (.y (Math|Vector|GetForwardVector (Math|Conversions|RotationFromXVector (* (Math|Vector|RotateVector (Math|Vector|MakeVector (.StickY (Class|PlayerController|GetInputAnalogStickState (LocalVariables|GetPlayerController) "CAS_LeftStick")) (.StickX (Class|PlayerController|GetInputAnalogStickState (LocalVariables|GetPlayerController) "CAS_LeftStick")) 0.0) (Transformation|GetActorRotation (LocalVariables|GetCameraManager))) (Math|Vector|MakeVector (Variables|Default|GetLeftRightScale) (Variables|Default|GetForwardBackwardScale) 0.0))))) 75.0) (.y (Transformation|GetActorLocation (LocalVariables|GetPlayerPawn)))) (+ (.z (Transformation|GetActorLocation (LocalVariables|GetPlayerPawn))) 75.0)) (LocalVariables|GetObjTypeArray) false 0 "None"))
    (if (not _returnvalue)
      (Class|TresGameBlueprintLibrary|BPTresActorMovetoLocation (LocalVariables|GetPlayerPawn) (LocalVariables|GetPlayerPawn) (+ (Transformation|GetActorLocation (LocalVariables|GetPlayerPawn)) (* (Math|Vector|RotateVector (Math|Vector|MakeVector (.StickY (Class|PlayerController|GetInputAnalogStickState (LocalVariables|GetPlayerController) "CAS_LeftStick")) (.StickX (Class|PlayerController|GetInputAnalogStickState (LocalVariables|GetPlayerController) "CAS_LeftStick")) 0.0) (Transformation|GetActorRotation (LocalVariables|GetCameraManager))) (Math|Vector|MakeVector (Variables|Default|GetLeftRightScale) (Variables|Default|GetForwardBackwardScale) 0.0))) (Variables|Default|GetTime) (Variables|Default|GetSnapFloor) (Variables|Default|GetRotation))
      (return false))))