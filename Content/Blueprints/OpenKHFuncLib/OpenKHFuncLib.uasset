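; OpenKHFuncLib is a helper function library for playing animation sequences based on distance to the lock-on target.
; AnimNotifyDistanceAnim reads the local Tres camera manager's lock-on target and calls PlayAnim when the given pawn is within a fixed range of its owner.
; PlayAnim calls AnimPlaySequence on player pawn 0 rather than using the passed mesh, and always returns false.
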(fn AnimNotifyDistanceAnim
  (params (Anim%20Sequence :type Anim%20Sequence%20Base%20Object%20Reference) (Pawn :type Tres%20Player%20Pawn%20Base%20Object%20Reference))
  (bind _returnvalue (Game|GetGameInstance))
  (bind _returnvalue_2 (Class|TresGameBlueprintLibrary|GetLocalTresCameraManager _returnvalue))
  (bind _m_lockontarget (Variables|/Script/TresGame.TresCameraManager|Getm_LockonTarget _returnvalue_2))
  (Utilities|IsValid _m_lockontarget
    (:Is%20Valid
      (if (< (Transformation|GetDistanceTo Pawn (Components|GetOwner _m_lockontarget)) 6.5e+02)
        (bind _return_value (CallFunction|PlayAnim (Variables|/Script/TresGame.TresCharPawnBase|GetMyMesh Pawn) Anim%20Sequence _returnvalue))
        (return _return_value)))))

(fn PlayAnim
  (params (Mesh%20Component :type Mesh%20Component%20Object%20Reference) (Anim%20Sequence :type Anim%20Sequence%20Base%20Object%20Reference))
  (Class|TresCharPawnBase|AnimPlaySequence (Class|TresGameBlueprintLibrary|GetTresPlayerPawnBase (Game|GetGameInstance)) (LocalVariables|GetAnimation) (LocalVariables|GetName) (LocalVariables|GetBlend%20Time) (LocalVariables|GetLoop) (LocalVariables|GetEffect%20Group) (LocalVariables|GetPlay%20Rate) (LocalVariables|GetRoot%20Translation) (LocalVariables|GetRoot%20Rotation) (LocalVariables|GetRoot%20Trans%20Scale%20XY) (LocalVariables|GetRoot%20Trans%20Scale%20Z))
  (return false))