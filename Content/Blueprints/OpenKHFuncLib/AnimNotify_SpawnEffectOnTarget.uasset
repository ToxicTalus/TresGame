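; Anim notify that spawns a particle effect on the player's current camera lock-on target.
; It reads the target from the local Tres camera manager and attaches the emitter to that actor's root component with configurable offset, rotation and scale.
; With no valid target, an optional fallback effect with its own settings spawns unattached at a set distance ahead of player 0 and height offset from them.
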(fn ReceivedNotify
  (params (MeshComp :type Skeletal%20Mesh%20Component%20Object%20Reference) (Animation :type Anim%20Sequence%20Base%20Object%20Reference))
  (bind _returnvalue (Class|TresGameBlueprintLibrary|GetLocalTresCameraManager))
  (Utilities|IsValid (Components|GetOwner (Variables|/Script/TresGame.TresCameraManager|Getm_LockonTarget _returnvalue))
    (:Is%20Valid
      (bind _returnvalue_2 (Effects|SpawnEmitterAttached (Variables|Default|GetParticle%20Effect) (Variables|/Script/Engine.Actor|GetRootComponent (Components|GetOwner (Variables|/Script/TresGame.TresCameraManager|Getm_LockonTarget _returnvalue))) "None" (Variables|Default|GetLocation%20Offset) (Variables|Default|GetRotation)))
      (Transformation|SetRelativeScale3D _returnvalue_2 (Variables|Default|GetScale))
      (return false))
    (:Is%20Not%20Valid
      (if (Variables|Default|GetNo%20Target%20Effect)
        (bind _returnvalue_3 (Class|TresGameBlueprintLibrary|GetTresPlayerPawnBase))
        (bind _returnvalue_4 (Effects|SpawnEmitteratLocation (Variables|Default|GetNT%20Particle%20Effect) (+ (Transformation|GetActorLocation _returnvalue_3) (Math|Vector|MakeVector (.x (* (Transformation|GetActorForwardVector _returnvalue_3) (Variables|Default|GetNT%20Distance%20From%20Player))) (.y (* (Transformation|GetActorForwardVector _returnvalue_3) (Variables|Default|GetNT%20Distance%20From%20Player))) (Variables|Default|GetNT%20Height%20From%20Player))) (Variables|Default|GetNT%20Rotation)))
        (Transformation|SetRelativeScale3D _returnvalue_4 (Variables|Default|GetNT%20Scale))
        (return false)))))